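; BP_NPC is an AI-controlled NPC in a hide-and-seek game that can be captured and freed.
; It finds the level's BP_CaptureZone on BeginPlay and caches it.
; Capture sets a captured flag, stops the AI controller's brain logic and teleports the NPC to that zone.
; Freeing clears the flag and restarts the logic, without moving the NPC.
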(event Custom|OnCaptured
  (Variables|Default|SetIsCaptured true)
  (AI|Logic|StopLogic (Variables|/Script/AIModule.AIController|GetBrainComponent (AI|GetAIController self)) "")
  (Transformation|Teleport (Transformation|GetActorLocation (Variables|Default|GetCaptureZone)) "0, 0, 0"))

(event Custom|OnFreed
  (Variables|Default|SetIsCaptured false)
  (Class|BrainComponent|RestartLogic (Variables|/Script/AIModule.AIController|GetBrainComponent (AI|GetAIController self))))

(event EventBeginPlay
  (bind _returnvalue (Actor|GetActorOfClass "/Game/BasicAI/HideAndSeek/LD/BP_CaptureZone.BP_CaptureZone_C"))
  (Variables|Default|SetCaptureZone _returnvalue))

(fn ConstructionScript)