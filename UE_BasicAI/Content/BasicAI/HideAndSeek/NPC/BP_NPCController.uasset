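; BP_NPCController is the AI controller for the hide-and-seek NPC, driving it through the BT_NPC behavior tree.
; On BeginPlay it runs the tree and seeds the blackboard with the player character as TargetActor and a BP_CaptureZone actor as CaptureZone.
; AI Perception updates feed HandleSightSense, which sets the TargetSpotted key to whether sight currently senses the player, ignoring other actors and senses.
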(event OnTargetPerceptionUpdated(AIPerception)
  (params (Actor :type Actor%20Object%20Reference) (Stimulus :type AI%20Stimulus%20Structure))
  (CallFunction|HandleSightSense Actor Stimulus))

(event EventBeginPlay
  (AI|RunBehaviorTree "/Game/BasicAI/HideAndSeek/BehaviourTree/BT_NPC.BT_NPC")
  (AI|Components|Blackboard|SetValueasObject (AI|GetBlackboard 0) (Utilities|Name|MakeLiteralName "TargetActor") (Game|GetPlayerCharacter 0))
  (bind _returnvalue (Actor|GetActorOfClass "/Game/BasicAI/HideAndSeek/LD/BP_CaptureZone.BP_CaptureZone_C"))
  (AI|Components|Blackboard|SetValueasObject (AI|GetBlackboard 0) (Utilities|Name|MakeLiteralName "CaptureZone") _returnvalue))

(fn ConstructionScript)

(fn HandleSightSense
  (params (Actor :type Actor%20Object%20Reference) (Stimulus :type AI%20Stimulus%20Structure))
  (bind _returnvalue (Class|AIPerceptionSystem|GetSenseClassforStimulus Stimulus))
  (if (== _returnvalue "/Script/AIModule.AISense_Sight")
    (if (== (Game|GetPlayerCharacter 0) Actor)
      (AI|Components|Blackboard|SetValueasBool (AI|GetBlackboard 0) (Utilities|Name|MakeLiteralName "TargetSpotted") (.bSuccessfullySensed (Utilities|Struct|BreakAIStimulus Stimulus))))))