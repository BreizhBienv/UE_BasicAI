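; BP_CaptureZone is a Blueprint for the hide-and-seek AI level that tracks which NPCs are captured.
; AddNPC and RemoveNPC maintain the CapturedNPC array, with AddUnique preventing duplicate entries.
; RandomCapturedNPC returns an entry by random index bounded by length minus one, so the last entry is never picked when several are held.
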(fn ConstructionScript)

(fn AddNPC
  (params (NPC :type BP%20NPC%20Object%20Reference))
  (Utilities|Array|AddUnique (Variables|Default|GetCapturedNPC) NPC))

(fn RemoveNPC
  (params (NPC :type BP%20NPC%20Object%20Reference))
  (Utilities|Array|RemoveItem (Variables|Default|GetCapturedNPC) NPC))

(fn RandomCapturedNPC
  (return (Utilities|Array|Get(acopy) (Variables|Default|GetCapturedNPC) (Math|Random|RandomInteger (- (Utilities|Array|Length (Variables|Default|GetCapturedNPC)) 1)))))