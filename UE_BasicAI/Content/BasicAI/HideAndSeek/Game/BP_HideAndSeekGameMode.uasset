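; Game mode for a hide-and-seek game that runs a timed Hiding phase followed by Seeking.
; BeginPlay broadcasts Hiding through the OnNewGamePhase dispatcher, whose phase-manager listener stores the current phase.
; Tick counts down and broadcasts Seeking at each expiry, resetting to the seeking timer, so Hiding never returns.
; The bound input-manager listener is empty; its logic for toggling player input by phase is disconnected.
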(event Custom|OnNewGamePhase_PhaseManager
  (params (NewPhase :type EGamePhase%20Enum :default "NewEnumerator0"))
  (Variables|Default|SetCurrentGamePhase NewPhase))

(event Custom|OnNewGamePhase_InputManager
  (params (NewPhase :type EGamePhase%20Enum :default "NewEnumerator0")))

(event EventBeginPlay
  (EventDispatchers|AssignOnNewGamePhase (delegate Custom|OnNewGamePhase_PhaseManager))
  (EventDispatchers|BindEventtoOnNewGamePhase (delegate Custom|OnNewGamePhase_InputManager))
  (Default|CallOnNewGamePhase "NewEnumerator0")
  (Variables|Default|SetCurrentTime (Math|Conversions|ToFloat(Integer) (Variables|Default|GetHidingTimer))))

(event EventTick
  (params (DeltaSeconds :type Float%20%28single-precision%29))
  (bind _output_get (Variables|Default|SetCurrentTime (- (Variables|Default|GetCurrentTime) DeltaSeconds)))
  (if (<= _output_get 0.0)
    (Default|CallOnNewGamePhase "NewEnumerator1")
    (Variables|Default|SetCurrentTime (Math|Conversions|ToFloat(Integer) (Variables|Default|GetSeekingTimer)))))

(fn ConstructionScript)